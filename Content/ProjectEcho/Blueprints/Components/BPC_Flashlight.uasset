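; Actor component that gives its owner a toggleable flashlight, which starts unowned and switched off.
; GiveFlashlight unlocks it, and ToggleFlashlight, also exposed as Toggle, flips the on state only once it is owned.
; ApplyLightState looks up the SpotLightComponent already on the owner rather than creating one, then sets its visibility, activation and intensity to match the state.
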(event `self.ReceiveBeginPlay`
  (set `self.bHasFlashlight` false)
  (set `self.bIsOn` false)
  (`self.EnsureLightComponent`)
  (`self.ApplyLightState`))

(fn `ApplyLightState`
  (`self.EnsureLightComponent`)
  (`/Engine/EditorBlueprintResources/StandardMacros.IsValid` (`self.FlashlightLight`)
    (:`Is Valid`
      (`SceneComponent.SetVisibility` (`self.FlashlightLight`) (`self.bIsOn`) false)
      (`self.SetActive` (`self.FlashlightLight`) (`self.bIsOn`) false)
      (`LightComponent.SetIntensity` (`self.FlashlightLight`) (select `bool` (`self.bIsOn`) :`false` 0.0 :`true` (`self.LightIntensity`))))))

(fn `EnsureLightComponent`
  (bind _returnvalue (`self.GetOwner`))
  (bind _returnvalue_2 (`Actor.GetComponentByClass` _returnvalue "/Script/Engine.SpotLightComponent"))
  (`/Engine/EditorBlueprintResources/StandardMacros.IsValid` _returnvalue
    (:`Is Valid`
      (`/Engine/EditorBlueprintResources/StandardMacros.IsValid` _returnvalue_2
        (:`Is Valid`
          (set `self.FlashlightLight` _returnvalue_2))))))

(fn `GiveFlashlight`
  (set `self.bHasFlashlight` true)
  (`self.EnsureLightComponent`)
  (`self.ApplyLightState`))

(fn `Toggle`
  (`self.ToggleFlashlight`))

(fn `ToggleFlashlight`
  (if (`self.bHasFlashlight`)
    (set `self.bIsOn` (not (`self.bIsOn`)))
    (`self.ApplyLightState`)))