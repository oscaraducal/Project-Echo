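; BP_InteractionComponent is an actor component that lets its owner interact with objects it is looking at.
; TryInteract sphere-traces on the Visibility channel from the owner's eyes view point along the view direction, using configurable distance and radius.
; Any hit actor becomes CurrentTarget; those implementing BPI_Interactable receive InteractMessage with the owner, gated by CanInteractMessage when RequireCanInteract is set.
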(fn `TryInteract`
  (bind _returnvalue (`self.GetOwner`))
  (bind (_outlocation _outrotation) (`Actor.GetActorEyesViewPoint` _returnvalue))
  (`/Engine/EditorBlueprintResources/StandardMacros.IsValid` _returnvalue
    (:`Is Valid`
      (bind (_outhit _returnvalue_2) (`KismetSystemLibrary.SphereTraceSingle` _outlocation (+ _outlocation (* (`KismetMathLibrary.Conv_RotatorToVector` _outrotation) (`self.TraceDistance`))) (`self.TraceRadius`) "TraceTypeQuery1"))
      (if _returnvalue_2
        (bind (_bblockinghit _binitialoverlap _time _distance _location _impactpoint _normal _impactnormal _physmat _hitactor) (`GameplayStatics.BreakHitResult` _outhit))
        (set `self.CurrentTarget` _hitactor)
        (if (`KismetSystemLibrary.DoesImplementInterface` _hitactor "/Game/ProjectEcho/Blueprints/Interfaces/BPI_Interactable.BPI_Interactable_C")
          (if (`self.bRequireCanInteract`)
            (bind _returnvalue_3 (message `/Game/ProjectEcho/Blueprints/Interfaces/BPI_Interactable.CanInteract` _hitactor _returnvalue))
            (if _returnvalue_3
              (message `/Game/ProjectEcho/Blueprints/Interfaces/BPI_Interactable.Interact` _hitactor _returnvalue))
            (else
              (message `/Game/ProjectEcho/Blueprints/Interfaces/BPI_Interactable.Interact` _hitactor _returnvalue))))))))