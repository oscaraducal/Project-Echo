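; BP_PASpeaker is a public-address speaker that reacts when power is restored.
; OnPowerRestored fires a one-shot sequence guarded by a Played flag, which BeginPlay resets.
; The sequence is placeholder print strings separated by short delays, describing static, a broken announcement burst and a cut to silence, with no audio played.
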(event `self.ReceiveBeginPlay`
  (set `self.bPlayed` false)
  (`KismetSystemLibrary.PrintString` "[PE012] PASpeaker idle"))

(event `OnPowerRestored`
  (if (not (`self.bPlayed`))
    (set `self.bPlayed` true)
    (`KismetSystemLibrary.PrintString` "[PE012][PA] Brief electrical static")
    (`KismetSystemLibrary.Delay` 0.2)
    (`KismetSystemLibrary.PrintString` "[PE012][PA] Incomplete announcement burst")
    (`KismetSystemLibrary.Delay` 0.15)
    (`KismetSystemLibrary.PrintString` "[PE012][PA] Signal cuts to silence")))

(fn `UserConstructionScript`)