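; BP_FuelCan is an interactable pickup that adds a fuel can item to the interacting actor's inventory.
; On Interact, it looks up the interactor's BPC_Inventory component, adds its ItemData, prints an acquisition message and destroys itself.
; Unconnected leftover logic, including a variant that sets an unlock-door objective through BPC_Objective, never runs.
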(event `self.ReceiveBeginPlay`
  (`parent.ReceiveBeginPlay`))

(event `self.Interact`
  (params (Interactor :type "Actor Object Reference"))
  (bind _returnvalue (`self.GetComponentByClass` Interactor "/Game/ProjectEcho/Blueprints/Components/BPC_Inventory.BPC_Inventory_C"))
  (`/Engine/EditorBlueprintResources/StandardMacros.IsValid` _returnvalue
    (:`Is Valid`
      (`/Game/ProjectEcho/Blueprints/Components/BPC_Inventory.AddItem` _returnvalue (`self.ItemData`))
      (`KismetSystemLibrary.PrintString` "Fuel Can acquired.")
      (`self.K2_DestroyActor` self))))

(fn `UserConstructionScript`
  (`parent.UserConstructionScript`))