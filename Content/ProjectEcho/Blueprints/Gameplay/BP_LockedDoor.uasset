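; BP_LockedDoor is an interactable door that only opens for actors carrying a required item.
; On Interact it asks the interactor's inventory component for RequiredItemID, printing a key-required message if the component or item is missing.
; With the item, it toggles open and closed by instantly rotating the whole actor 90 degrees in yaw.
; Each opening also calls CompleteObjective on the interactor's objective component, if present.
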(event `/Game/ProjectEcho/Blueprints/Interfaces/BPI_Interactable.Interact`
  (params (Interactor :type "Actor Object Reference"))
  (bind _returnvalue (`self.GetComponentByClass` Interactor "/Game/ProjectEcho/Blueprints/Components/BP_InventoryComponent.BP_InventoryComponent_C"))
  (bind _returnvalue_2 (`self.GetComponentByClass` Interactor "/Game/ProjectEcho/Blueprints/Components/BP_ObjectiveComponent.BP_ObjectiveComponent_C"))
  (bind _returnvalue_3 (not (`self.IsOpen`)))
  (`/Engine/EditorBlueprintResources/StandardMacros.IsValid` _returnvalue
    (:`Is Valid`
      (bind _returnvalue_4 (`/Game/ProjectEcho/Blueprints/Components/BP_InventoryComponent.HasItem` _returnvalue (`self.RequiredItemID`)))
      (if _returnvalue_4
        (if _returnvalue_3
          (set `self.IsOpen` _returnvalue_3)
          (`self.K2_AddActorLocalRotation` (`KismetMathLibrary.MakeRotator` 0.0 0.0 90.0))
          (`/Engine/EditorBlueprintResources/StandardMacros.IsValid` _returnvalue_2
            (:`Is Valid`
              (`/Game/ProjectEcho/Blueprints/Components/BP_ObjectiveComponent.CompleteObjective` _returnvalue_2)))
          (else
            (set `self.IsOpen` false)
            (`self.K2_AddActorLocalRotation` (`KismetMathLibrary.MakeRotator` 0.0 0.0 -90.0))))
        (else
          (`KismetSystemLibrary.PrintString` "Requires Facility Key."))))
    (:`Is Not Valid`
      (`KismetSystemLibrary.PrintString` "Requires Facility Key."))))

(fn `UserConstructionScript`)