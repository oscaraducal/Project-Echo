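; BP_PoweredDoor is a door that starts locked and becomes usable once power is restored.
; BeginPlay sets it locked and closed, and OnPowerRestored clears the lock.
; Interact logs a refusal while locked, otherwise it toggles IsOpen.
; The door has only state and debug prints, with no movement logic, and its OPEN and CLOSED messages are inverted relative to IsOpen.
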(event `self.ReceiveBeginPlay`
  (set `self.bIsLocked` true)
  (set `self.bIsOpen` false)
  (`KismetSystemLibrary.PrintString` "[PE011] PoweredDoor locked"))

(event `OnPowerRestored`
  (set `self.bIsLocked` false)
  (`KismetSystemLibrary.PrintString` "[PE011] PoweredDoor UNLOCKED"))

(event `/Game/ProjectEcho/Blueprints/Interfaces/BPI_Interactable.Interact`
  (params (Interactor :type "Actor Object Reference"))
  (bind _bisopen (`self.bIsOpen`))
  (if (`self.bIsLocked`)
    (`KismetSystemLibrary.PrintString` "[PE011] Door locked / no power")
    (else
      (set `self.bIsOpen` (not _bisopen))
      (if (not _bisopen)
        (`KismetSystemLibrary.PrintString` "[PE011] PoweredDoor OPEN")
        (else
          (`KismetSystemLibrary.PrintString` "[PE011] PoweredDoor CLOSED"))))))

(fn `UserConstructionScript`
  (`parent.UserConstructionScript`))