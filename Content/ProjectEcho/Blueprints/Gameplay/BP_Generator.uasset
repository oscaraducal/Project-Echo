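; Interactable generator that restores power once the player supplies a fuel can, driven by an integer state for empty, fueled and running.
; The first interaction takes a FuelCan from the interactor's inventory component, or sets a "Find Fuel" objective if none is held.
; Interacting when fueled starts a short timer to FinishGeneratorStart, which fires OnPowerRestored and completes the cached interactor's objective.
; Feedback is only PrintString messages.
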(event `self.ReceiveBeginPlay`
  (`parent.ReceiveBeginPlay`))

(event `/Game/ProjectEcho/Blueprints/Interfaces/BPI_Interactable.Interact`
  (params (Interactor :type "Actor Object Reference"))
  (bind _returnvalue (`self.GetComponentByClass` Interactor "/Game/ProjectEcho/Blueprints/Components/BP_InventoryComponent.BP_InventoryComponent_C"))
  (bind _returnvalue_2 (`self.GetComponentByClass` Interactor "/Game/ProjectEcho/Blueprints/Components/BP_ObjectiveComponent.BP_ObjectiveComponent_C"))
  (bind _generatorstate (`self.GeneratorState`))
  (if (== _generatorstate 2)
    (`KismetSystemLibrary.PrintString` "Generator already running.")
    (elif (== _generatorstate 0)
      (`/Engine/EditorBlueprintResources/StandardMacros.IsValid` _returnvalue
        (:`Is Valid`
          (bind _returnvalue_3 (`/Game/ProjectEcho/Blueprints/Components/BP_InventoryComponent.HasItem` _returnvalue "FuelCan"))
          (if _returnvalue_3
            (`/Game/ProjectEcho/Blueprints/Components/BP_InventoryComponent.RemoveItem` _returnvalue "FuelCan")
            (set `self.HasFuel` true)
            (set `self.GeneratorState` 1)
            (`KismetSystemLibrary.PrintString` "Fuel inserted.")
            (else
              (`KismetSystemLibrary.PrintString` "Generator requires fuel.")
              (`/Engine/EditorBlueprintResources/StandardMacros.IsValid` _returnvalue_2
                (:`Is Valid`
                  (`/Game/ProjectEcho/Blueprints/Components/BP_ObjectiveComponent.SetObjective` _returnvalue_2 "Find Fuel"))))))
        (:`Is Not Valid`
          (`KismetSystemLibrary.PrintString` "Generator requires fuel.")))
      (else
        (set `self.CachedInteractor` Interactor)
        (`KismetSystemLibrary.PrintString` "Generator starting...")
        (`KismetSystemLibrary.K2_SetTimer` self "FinishGeneratorStart" 2.0)))))

(event `OnPowerRestored_Event`)

(fn `FinishGeneratorStart`
  (bind _returnvalue (`self.GetComponentByClass` (`self.CachedInteractor`) "/Game/ProjectEcho/Blueprints/Components/BP_ObjectiveComponent.BP_ObjectiveComponent_C"))
  (set `self.GeneratorState` 2)
  (set `self.PowerRestored` true)
  (`self.OnPowerRestored`)
  (`KismetSystemLibrary.PrintString` "Power restored.")
  (`/Engine/EditorBlueprintResources/StandardMacros.IsValid` _returnvalue
    (:`Is Valid`
      (`/Game/ProjectEcho/Blueprints/Components/BP_ObjectiveComponent.CompleteObjective` _returnvalue))))

(fn `UserConstructionScript`
  (`parent.UserConstructionScript`))