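; Power manager actor that triggers the world's response when generator power is restored.
; BeginPlay binds generators to an empty handler and stores the last one, so Tick polling of its PowerRestored flag actually triggers the response.
; A one-shot HandlePowerRestored notifies lights, doors, ambience, vents, PA speakers and activity hints, then advances the player's objective to the security door.
; Leftover unreachable binding chains and stub events remain.
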(event `self.ReceiveBeginPlay`
  (`KismetSystemLibrary.PrintString` "[PE012] PowerManager ready")
  (bind _outactors (`GameplayStatics.GetAllActorsOfClass` "/Game/ProjectEcho/Blueprints/Gameplay/BP_Generator.BP_Generator_C"))
  (for _array_element _outactors
    (set `self.BoundGeneratorActor` _array_element)
    (bind _asbp_generator (cast `/Game/ProjectEcho/Blueprints/Gameplay/BP_Generator` _array_element)
      (:`then`
        (set `self.BoundGenerator` _asbp_generator)
        (add `/Game/ProjectEcho/Blueprints/Gameplay/BP_Generator.OnPowerRestored` _asbp_generator (delegate `OnPowerRestored_Event_13`))
        (`KismetSystemLibrary.PrintString` "[PE012] Bound generator OnPowerRestored"))
      (:`CastFailed`
        (`KismetSystemLibrary.PrintString` "[PE012] Generator cast failed")))))

(event `OnPowerRestored_Event_0`)

(event `OnPowerRestored_Event_3`)

(event `OnPowerRestored_Event_5`)

(event `OnPowerRestored_Event_7`)

(event `OnPowerRestored_Event_8`)

(event `OnPowerRestored_Event_9`)

(event `OnPowerRestored_Event_10`)

(event `OnPowerRestored_Event_11`)

(event `OnPowerRestored_Event_12`)

(event `OnPowerRestored_Event_14`)

(event `OnPowerRestored_Event_15`)

(event `OnPowerRestored_Event`
  (`self.HandlePowerRestored`))

(event `HandlePowerRestored`
  (bind _returnvalue (`self.GetComponentByClass` (`GameplayStatics.GetPlayerPawn` 0) "/Game/ProjectEcho/Blueprints/Components/BP_ObjectiveComponent.BP_ObjectiveComponent_C"))
  (if (not (`self.HasHandledPower`))
    (set `self.HasHandledPower` true)
    (`KismetSystemLibrary.PrintString` "[PE012] Power Manager received PowerRestored - world response begin")
    (bind _outactors (`GameplayStatics.GetAllActorsOfClass` "/Game/ProjectEcho/Blueprints/Gameplay/BP_EmergencyLight.BP_EmergencyLight_C"))
    (for _array_element _outactors
      (`/Game/ProjectEcho/Blueprints/Gameplay/BP_EmergencyLight.OnPowerRestored` _array_element))
    (bind _outactors_2 (`GameplayStatics.GetAllActorsOfClass` "/Game/ProjectEcho/Blueprints/Gameplay/BP_PoweredDoor.BP_PoweredDoor_C"))
    (for _array_element_2 _outactors_2
      (`/Game/ProjectEcho/Blueprints/Gameplay/BP_PoweredDoor.OnPowerRestored` _array_element_2))
    (bind _outactors_3 (`GameplayStatics.GetAllActorsOfClass` "/Game/ProjectEcho/Blueprints/Gameplay/BP_PowerAmbientFeedback.BP_PowerAmbientFeedback_C"))
    (for _array_element_3 _outactors_3
      (`/Game/ProjectEcho/Blueprints/Gameplay/BP_PowerAmbientFeedback.OnPowerRestored` _array_element_3))
    (bind _outactors_4 (`GameplayStatics.GetAllActorsOfClass` "/Game/ProjectEcho/Blueprints/Gameplay/Power/BP_VentilationUnit.BP_VentilationUnit_C"))
    (for _array_element_4 _outactors_4
      (`/Game/ProjectEcho/Blueprints/Gameplay/Power/BP_VentilationUnit.OnPowerRestored` _array_element_4))
    (bind _outactors_5 (`GameplayStatics.GetAllActorsOfClass` "/Game/ProjectEcho/Blueprints/Gameplay/Power/BP_PASpeaker.BP_PASpeaker_C"))
    (for _array_element_5 _outactors_5
      (`/Game/ProjectEcho/Blueprints/Gameplay/Power/BP_PASpeaker.OnPowerRestored` _array_element_5))
    (bind _outactors_6 (`GameplayStatics.GetAllActorsOfClass` "/Game/ProjectEcho/Blueprints/Gameplay/Power/BP_DistantActivityHint.BP_DistantActivityHint_C"))
    (for _array_element_6 _outactors_6
      (`/Game/ProjectEcho/Blueprints/Gameplay/Power/BP_DistantActivityHint.OnPowerRestored` _array_element_6))
    (`/Engine/EditorBlueprintResources/StandardMacros.IsValid` _returnvalue
      (:`Is Valid`
        (`/Game/ProjectEcho/Blueprints/Components/BP_ObjectiveComponent.CompleteObjective` _returnvalue)
        (`/Game/ProjectEcho/Blueprints/Components/BP_ObjectiveComponent.SetObjective` _returnvalue "Proceed through the powered security door.")
        (`KismetSystemLibrary.PrintString` "[PE012] Objective set: Proceed through the powered security door."))
      (:`Is Not Valid`
        (`KismetSystemLibrary.PrintString` "[PE012] ObjectiveComponent missing")))))

(event `CustomEvent`)

(event `CustomEvent_0`)

(event `CustomEvent_1`)

(event `self.ReceiveTick`
  (params (DeltaSeconds :type "Float (single-precision)"))
  (bind _boundgenerator (`self.BoundGenerator`))
  (if (not (`self.HasHandledPower`))
    (`/Engine/EditorBlueprintResources/StandardMacros.IsValid` _boundgenerator
      (:`Is Valid`
        (if (`/Game/ProjectEcho/Blueprints/Gameplay/BP_Generator.PowerRestored` _boundgenerator)
          (`self.HandlePowerRestored`))))))

(event `OnPowerRestored_Event_1`
  (`self.HandlePowerRestored`))

(event `OnPowerRestored_Event_2`
  (`self.HandlePowerRestored`))

(event `OnPowerRestored_Event_4`)

(event `OnPowerRestored_Event_6`
  (`self.HandlePowerRestored`))

(event `OnPowerRestored_Event_13`)

(fn `UserConstructionScript`)