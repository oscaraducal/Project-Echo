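; BP_PowerAmbientFeedback is an actor that stands in for the ambient audio feedback when facility power is restored.
; Its OnPowerRestored event uses a Played flag to run only once.
; It prints a timed series of tagged debug messages, separated by short delays, naming hum, ventilation, buzz, ambience and emergency-system cues.
; No sounds are actually played, and BeginPlay and the construction script are empty.
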(event `self.ReceiveBeginPlay`)

(event `OnPowerRestored`
  (if (not (`self.bPlayed`))
    (set `self.bPlayed` true)
    (`KismetSystemLibrary.PrintString` "[PE011][Audio] Power hum")
    (`KismetSystemLibrary.Delay` 0.4)
    (`KismetSystemLibrary.PrintString` "[PE011][Audio] Ventilation restored")
    (`KismetSystemLibrary.Delay` 0.4)
    (`KismetSystemLibrary.PrintString` "[PE011][Audio] Electrical buzz")
    (`KismetSystemLibrary.Delay` 0.4)
    (`KismetSystemLibrary.PrintString` "[PE011][Audio] Facility ambience")
    (`KismetSystemLibrary.PrintString` "[PE011][Audio] Emergency systems online")))

(fn `UserConstructionScript`)