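; BP_NotePickup is an interactable note actor that shows its title and body in a WBP_Note widget.
; Each Interact creates and displays a fresh widget, so the note can be reread.
; The first read sets a Collected flag and, if the interactor has a BP_ObjectiveComponent, sets its objective to locating the Facility Key.
; GetInteractionText switches the prompt from reading to rereading once collected.
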(event `/Game/ProjectEcho/Blueprints/Interfaces/BPI_Interactable.Interact`
  (params (Interactor :type "Actor Object Reference"))
  (bind _returnvalue (`self.GetComponentByClass` Interactor "/Game/ProjectEcho/Blueprints/Components/BP_ObjectiveComponent.BP_ObjectiveComponent_C"))
  (bind _returnvalue_2 (`|CreateWidget` "/Game/ProjectEcho/Blueprints/UI/WBP_Note.WBP_Note_C" (`GameplayStatics.GetPlayerController` 0)))
  (`/Game/ProjectEcho/Blueprints/UI/WBP_Note.SetupNote` _returnvalue_2 (`self.NoteTitle`) (`self.NoteBody`))
  (`UserWidget.AddToViewport` _returnvalue_2 0)
  (if (not (`self.bCollected`))
    (set `self.bCollected` true)
    (`KismetSystemLibrary.PrintString` "[PE008] Note displayed")
    (`/Engine/EditorBlueprintResources/StandardMacros.IsValid` _returnvalue
      (:`Is Valid`
        (`/Game/ProjectEcho/Blueprints/Components/BP_ObjectiveComponent.SetObjective` _returnvalue "Locate the Facility Key")))))

(fn `GetInteractionText`
  (returns (ReturnValue :type Text))
  (if (`self.bCollected`)
    (return "Read again")
    (else
      (return "Read note"))))

(fn `UserConstructionScript`)