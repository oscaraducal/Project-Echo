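; Player character Blueprint that turns Enhanced Input actions into movement, look, jump, sprint, interaction and flashlight toggling.
; Movement follows actor yaw, look applies per-axis sensitivity with inverted pitch input, and sprint swaps max walk speed while held.
; Interaction and flashlight actions delegate to components, and BeginPlay sets a "Find a flashlight" objective through the objective component.
; Sprint-check, movement-state and movement-noise functions are empty stubs.
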(event `self.ReceiveBeginPlay`
  (bind _returnvalue (`self.GetComponentByClass` self "/Game/ProjectEcho/Blueprints/Components/BP_ObjectiveComponent.BP_ObjectiveComponent_C"))
  (`self.ApplyWalkSpeed`)
  (`/Engine/EditorBlueprintResources/StandardMacros.IsValid` _returnvalue
    (:`Is Valid`
      (`/Game/ProjectEcho/Blueprints/Components/BP_ObjectiveComponent.SetObjective` _returnvalue "Find a flashlight"))))

(event `EnhancedInput|/Game/ProjectEcho/Input/IA_Move`
  (params (ActionValue :type "Vector2D Structure") (ElapsedSeconds :type "Float (double-precision)") (TriggeredSeconds :type "Float (double-precision)") (InputAction :type "InputAction Object Reference" :default "/Game/ProjectEcho/Input/IA_Move.IA_Move"))
  (:`Triggered`
    (`self.HandleMoveInput` ActionValue)))

(event `EnhancedInput|/Game/ProjectEcho/Input/IA_Look`
  (params (ActionValue :type "Vector2D Structure") (ElapsedSeconds :type "Float (double-precision)") (TriggeredSeconds :type "Float (double-precision)") (InputAction :type "InputAction Object Reference" :default "/Game/ProjectEcho/Input/IA_Look.IA_Look"))
  (:`Triggered`
    (`self.HandleLookInput` ActionValue)))

(event `EnhancedInput|/Game/ProjectEcho/Input/IA_Jump`
  (params (ActionValue :type Boolean) (ElapsedSeconds :type "Float (double-precision)") (TriggeredSeconds :type "Float (double-precision)") (InputAction :type "InputAction Object Reference" :default "/Game/ProjectEcho/Input/IA_Jump.IA_Jump"))
  (:`Started`
    (`self.Jump`))
  (:`Completed`
    (`self.StopJumping`)))

(event `EnhancedInput|/Game/ProjectEcho/Input/IA_Sprint`
  (params (ActionValue :type Boolean) (ElapsedSeconds :type "Float (double-precision)") (TriggeredSeconds :type "Float (double-precision)") (InputAction :type "InputAction Object Reference" :default "/Game/ProjectEcho/Input/IA_Sprint.IA_Sprint"))
  (:`Started`
    (`self.ApplySprintSpeed`))
  (:`Completed`
    (`self.ApplyWalkSpeed`)))

(event `EnhancedInput|/Game/ProjectEcho/Input/IA_Interact`
  (params (ActionValue :type Boolean) (ElapsedSeconds :type "Float (double-precision)") (TriggeredSeconds :type "Float (double-precision)") (InputAction :type "InputAction Object Reference" :default "/Game/ProjectEcho/Input/IA_Interact.IA_Interact"))
  (:`Started`
    (`/Game/ProjectEcho/Blueprints/Components/BP_InteractionComponent.TryInteract` (`self.InteractionComponent`))))

(event `EnhancedInput|/Game/ProjectEcho/Input/IA_Flashlight`
  (params (ActionValue :type Boolean) (ElapsedSeconds :type "Float (double-precision)") (TriggeredSeconds :type "Float (double-precision)") (InputAction :type "InputAction Object Reference" :default "/Game/ProjectEcho/Input/IA_Flashlight.IA_Flashlight"))
  (:`Started`
    (`/Game/ProjectEcho/Blueprints/Components/BP_FlashlightComponent.ToggleFlashlight` (`self.GetComponentByClass` "/Game/ProjectEcho/Blueprints/Components/BP_FlashlightComponent.BP_FlashlightComponent_C"))))

(fn `ApplySprintSpeed`
  (set `CharacterMovementComponent.MaxWalkSpeed` (`self.SprintSpeed`) (`self.CharacterMovement`)))

(fn `ApplyWalkSpeed`
  (set `CharacterMovementComponent.MaxWalkSpeed` (`self.WalkSpeed`) (`self.CharacterMovement`)))

(fn `CanStartSprint`)

(fn `GenerateMovementNoise`)

(fn `HandleLookInput`
  (params (LookAxis :type "Vector2D Structure"))
  (`self.AddControllerYawInput` (* (.x (`KismetMathLibrary.Conv_Vector2DToVector` LookAxis)) (`self.HorizontalSensitivity`)))
  (`self.AddControllerPitchInput` (* (.y (`KismetMathLibrary.Conv_Vector2DToVector` LookAxis)) (- 0.0 (`self.VerticalSensitivity`)))))

(fn `HandleMoveInput`
  (params (MoveAxis :type "Vector2D Structure"))
  (bind _returnvalue (`KismetMathLibrary.Conv_Vector2DToVector` MoveAxis))
  (bind _returnvalue_2 (`KismetMathLibrary.MakeRotator` 0.0 0.0 (.yaw (`self.K2_GetActorRotation` self))))
  (`self.AddMovementInput` self (`KismetMathLibrary.GetForwardVector` _returnvalue_2) (.y _returnvalue) false)
  (`self.AddMovementInput` self (`KismetMathLibrary.GetRightVector` _returnvalue_2) (.x _returnvalue) false))

(fn `OnMovementStateChanged`)

(fn `StartSprint`)

(fn `StopSprint`)

(fn `UserConstructionScript`)