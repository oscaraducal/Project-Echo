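; Dev sandbox smoke test that auto-runs on BeginPlay to exercise Project Echo's player and interaction systems.
; After a short delay it checks the player pawn, then invokes movement, look and sprint.
; It calls Interact on every placed pickup, door and generator, re-interacts generators to activate them, then toggles the flashlight.
; PASS prints only confirm calls were made, not their results; its own Interact is an empty stub.
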(event `self.ReceiveBeginPlay`
  (bind _returnvalue (`GameplayStatics.GetPlayerPawn` 0))
  (`KismetSystemLibrary.PrintString` "[PE013B] Validator BeginPlay")
  (`KismetSystemLibrary.RetriggerableDelay` 0.75)
  (`/Engine/EditorBlueprintResources/StandardMacros.IsValid` _returnvalue
    (:`Is Valid`
      (`KismetSystemLibrary.PrintString` "[PE013B] PASS Spawn: player pawn valid")
      (bind _asbp_player_character (cast `/Game/ProjectEcho/Gameplay/Characters/BP_PlayerCharacter` _returnvalue)
        (:`then`
          (`Pawn.AddMovementInput` _asbp_player_character (`KismetMathLibrary.MakeVector` 1.0) 1.0 false)
          (`/Game/ProjectEcho/Gameplay/Characters/BP_PlayerCharacter.HandleLookInput` _asbp_player_character (`KismetMathLibrary.MakeVector2D` 0.05))
          (`/Game/ProjectEcho/Gameplay/Characters/BP_PlayerCharacter.StartSprint` _asbp_player_character)
          (`KismetSystemLibrary.PrintString` "[PE013B] PASS Movement/Look/Sprint APIs invoked")
          (bind _outactors (`GameplayStatics.GetAllActorsOfClass` "/Game/ProjectEcho/Gameplay/Inventory/BP_FlashlightPickup.BP_FlashlightPickup_C"))
          (bind _outactors_2 (`GameplayStatics.GetAllActorsOfClass` "/Game/ProjectEcho/Gameplay/Interaction/BP_Door.BP_Door_C"))
          (bind _outactors_3 (`GameplayStatics.GetAllActorsOfClass` "/Game/ProjectEcho/Gameplay/Inventory/BP_FuelCan.BP_FuelCan_C"))
          (bind _outactors_4 (`GameplayStatics.GetAllActorsOfClass` "/Game/ProjectEcho/Gameplay/Inventory/BP_KeyItemPickup.BP_KeyItemPickup_C"))
          (bind _outactors_5 (`GameplayStatics.GetAllActorsOfClass` "/Game/ProjectEcho/Gameplay/Interaction/BP_NotePickup.BP_NotePickup_C"))
          (bind _outactors_6 (`GameplayStatics.GetAllActorsOfClass` "/Game/ProjectEcho/Gameplay/Power/BP_Generator.BP_Generator_C"))
          (for _array_element _outactors
            (`/Game/ProjectEcho/Gameplay/Interaction/BP_InteractableBase.Interact` _array_element _asbp_player_character)
            (`KismetSystemLibrary.PrintString` "[PE013B] PASS Interaction/Inventory: Flashlight Interact"))
          (for _array_element_2 _outactors_2
            (`/Game/ProjectEcho/Gameplay/Interaction/BP_InteractableBase.Interact` _array_element_2 _asbp_player_character)
            (`KismetSystemLibrary.PrintString` "[PE013B] PASS Interaction: Door Interact"))
          (for _array_element_3 _outactors_5
            (`/Game/ProjectEcho/Gameplay/Interaction/BP_InteractableBase.Interact` _array_element_3 _asbp_player_character)
            (`KismetSystemLibrary.PrintString` "[PE013B] PASS Notes: NotePickup Interact (NoteReader)"))
          (for _array_element_4 _outactors_4
            (`/Game/ProjectEcho/Gameplay/Interaction/BP_InteractableBase.Interact` _array_element_4 _asbp_player_character)
            (`KismetSystemLibrary.PrintString` "[PE013B] PASS Inventory: KeyItem Interact"))
          (for _array_element_5 _outactors_3
            (`/Game/ProjectEcho/Gameplay/Interaction/BP_InteractableBase.Interact` _array_element_5 _asbp_player_character)
            (`KismetSystemLibrary.PrintString` "[PE013B] PASS Inventory: FuelCan Interact"))
          (for _array_element_6 _outactors_6
            (`/Game/ProjectEcho/Gameplay/Interaction/BP_InteractableBase.Interact` _array_element_6 _asbp_player_character)
            (`KismetSystemLibrary.PrintString` "[PE013B] PASS Generator: fuel insert Interact"))
          (`KismetSystemLibrary.RetriggerableDelay` 0.5)
          (for _array_element_7 _outactors_6
            (`/Game/ProjectEcho/Gameplay/Interaction/BP_InteractableBase.Interact` _array_element_7 _asbp_player_character)
            (`KismetSystemLibrary.PrintString` "[PE013B] PASS Generator: activate Interact"))
          (`KismetSystemLibrary.RetriggerableDelay` 2.5)
          (bind _returnvalue_2 (`self.GetComponentByClass` _asbp_player_character "/Game/ProjectEcho/Gameplay/Systems/BPC_Flashlight.BPC_Flashlight_C"))
          (`/Engine/EditorBlueprintResources/StandardMacros.IsValid` _returnvalue_2
            (:`Is Valid`
              (`/Game/ProjectEcho/Gameplay/Systems/BPC_Flashlight.ToggleFlashlight` _returnvalue_2)
              (`KismetSystemLibrary.PrintString` "[PE013B] PASS Flashlight toggle")
              (`KismetSystemLibrary.PrintString` "[PE013B] Validator sequence complete"))
            (:`Is Not Valid`
              (`KismetSystemLibrary.PrintString` "[PE013B] FAIL Flashlight component missing")
              (`KismetSystemLibrary.PrintString` "[PE013B] Validator sequence complete"))))
        (:`CastFailed`
          (`KismetSystemLibrary.PrintString` "[PE013B] FAIL Spawn: pawn is not BP_PlayerCharacter"))))
    (:`Is Not Valid`
      (`KismetSystemLibrary.PrintString` "[PE013B] FAIL Spawn: no player pawn"))))

(event `self.Interact`
  (params (Interactor :type "Actor Object Reference")))

(fn `CanInteract`
  (params (Interactor :type "Actor Object Reference"))
  (returns (ReturnValue :type Boolean))
  (return true))

(fn `GetInteractionText`
  (returns (ReturnValue :type Text))
  (return "Interact"))

(fn `UserConstructionScript`)