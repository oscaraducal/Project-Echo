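; Interactable "Reset Puzzle" actor that restores the Generator Annex power puzzle to its starting state.
; ResetWorldState finds actors by class and directly writes door, light, generator, feedback and note variables, calling a reset function only on witness hints.
; ResetPlayerState removes the fuel can item and restores the starting objective, also set at BeginPlay.
; FinishPuzzleReset destroys all fuel cans, optionally respawning one at FuseSpawnPoint or, failing that, this actor.
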(event `self.ReceiveBeginPlay`
  (bind _returnvalue (`self.GetComponentByClass` (`GameplayStatics.GetPlayerPawn` 0) "/Game/ProjectEcho/Gameplay/Objectives/BPC_Objective.BPC_Objective_C"))
  (`/Engine/EditorBlueprintResources/StandardMacros.IsValid` _returnvalue
    (:`Is Valid`
      (`/Game/ProjectEcho/Gameplay/Objectives/BPC_Objective.SetObjective` _returnvalue "Investigate the main power plant")
      (`KismetSystemLibrary.PrintString` "[PE018] Generator Annex ready"))
    (:`Is Not Valid`
      (`KismetSystemLibrary.PrintString` "[PE018] ObjectiveComponent missing at BeginPlay"))))

(event `self.Interact`
  (params (Interactor :type "Actor Object Reference"))
  (`self.ResetWorldState`)
  (`self.ResetPlayerState`)
  (`self.FinishPuzzleReset`))

(fn `CanInteract`
  (params (Interactor :type "Actor Object Reference"))
  (returns (ReturnValue :type Boolean))
  (return true))

(fn `CompleteSliceReset`
  (`self.ResetWorldState`)
  (`self.ResetPlayerState`)
  (`self.FinishPuzzleReset`)
  (`KismetSystemLibrary.PrintString` "[PE018] Slice world state fully reset"))

(fn `FinishPuzzleReset`
  (bind _fusespawnpoint (`self.FuseSpawnPoint`))
  (bind _outactors (`GameplayStatics.GetAllActorsOfClass` "/Game/ProjectEcho/Gameplay/Inventory/BP_FuelCan.BP_FuelCan_C"))
  (for _array_element _outactors
    (`self.K2_DestroyActor` _array_element))
  (if (`self.bRespawnFuse`)
    (`/Engine/EditorBlueprintResources/StandardMacros.IsValid` _fusespawnpoint
      (:`Is Valid`
        (`|SpawnActorFromClass` "/Game/ProjectEcho/Gameplay/Inventory/BP_FuelCan.BP_FuelCan_C" (`self.GetTransform` _fusespawnpoint) "AlwaysSpawn" "MultiplyWithRoot" null null)
        (`KismetSystemLibrary.PrintString` "[PE018] FuelCan respawned")
        (`KismetSystemLibrary.PrintString` "[PE018] SliceReset complete"))
      (:`Is Not Valid`
        (`|SpawnActorFromClass` "/Game/ProjectEcho/Gameplay/Inventory/BP_FuelCan.BP_FuelCan_C" (`self.GetTransform`) "AlwaysSpawn" "MultiplyWithRoot" null null)
        (`KismetSystemLibrary.PrintString` "[PE018] FuelCan respawned at reset button")
        (`KismetSystemLibrary.PrintString` "[PE018] SliceReset complete")))
    (else
      (`KismetSystemLibrary.PrintString` "[PE018] SliceReset complete"))))

(fn `GetInteractionText`
  (returns (ReturnValue :type Text))
  (return "Reset Puzzle"))

(fn `ResetPlayerState`
  (bind _returnvalue (`GameplayStatics.GetPlayerPawn` 0))
  (bind _returnvalue_2 (`self.GetComponentByClass` _returnvalue "/Game/ProjectEcho/Gameplay/Inventory/BPC_Inventory.BPC_Inventory_C"))
  (bind _returnvalue_3 (`self.GetComponentByClass` _returnvalue "/Game/ProjectEcho/Gameplay/Objectives/BPC_Objective.BPC_Objective_C"))
  (`/Engine/EditorBlueprintResources/StandardMacros.IsValid` _returnvalue_2
    (:`Is Valid`
      (`/Game/ProjectEcho/Gameplay/Inventory/BPC_Inventory.RemoveItem` _returnvalue_2 (`KismetStringLibrary.Conv_StringToName` "FuelCan"))
      (`/Engine/EditorBlueprintResources/StandardMacros.IsValid` _returnvalue_3
        (:`Is Valid`
          (`/Game/ProjectEcho/Gameplay/Objectives/BPC_Objective.SetObjective` _returnvalue_3 "Investigate the main power plant"))))
    (:`Is Not Valid`
      (`/Engine/EditorBlueprintResources/StandardMacros.IsValid` _returnvalue_3
        (:`Is Valid`
          (`/Game/ProjectEcho/Gameplay/Objectives/BPC_Objective.SetObjective` _returnvalue_3 "Investigate the main power plant"))))))

(fn `ResetWorldState`
  (bind _returnvalue (`self.GetComponentByClass` (`GameplayStatics.GetPlayerPawn` 0) "/Game/ProjectEcho/Gameplay/Objectives/BPC_Objective.BPC_Objective_C"))
  (bind _outactors (`GameplayStatics.GetAllActorsOfClass` "/Game/ProjectEcho/Gameplay/Power/BP_PoweredDoor.BP_PoweredDoor_C"))
  (for _array_element _outactors
    (set `/Game/ProjectEcho/Gameplay/Power/BP_PoweredDoor.bIsLocked` true _array_element)
    (set `/Game/ProjectEcho/Gameplay/Power/BP_PoweredDoor.bIsOpen` false _array_element))
  (bind _outactors_2 (`GameplayStatics.GetAllActorsOfClass` "/Game/ProjectEcho/Gameplay/Power/BP_EmergencyLight.BP_EmergencyLight_C"))
  (for _array_element_2 _outactors_2
    (set `/Game/ProjectEcho/Gameplay/Power/BP_EmergencyLight.bPoweredOn` false _array_element_2))
  (bind _outactors_3 (`GameplayStatics.GetAllActorsOfClass` "/Game/ProjectEcho/Gameplay/Power/BP_WitnessSilhouetteHint.BP_WitnessSilhouetteHint_C"))
  (for _array_element_3 _outactors_3
    (`/Game/ProjectEcho/Gameplay/Power/BP_WitnessSilhouetteHint.ResetPresence` _array_element_3))
  (bind _outactors_4 (`GameplayStatics.GetAllActorsOfClass` "/Game/ProjectEcho/Gameplay/Power/BP_PowerManager.BP_PowerManager_C"))
  (for _array_element_4 _outactors_4
    (set `/Game/ProjectEcho/Gameplay/Power/BP_PowerManager.HasHandledPower` false _array_element_4))
  (bind _outactors_5 (`GameplayStatics.GetAllActorsOfClass` "/Game/ProjectEcho/Gameplay/Power/BP_PowerAmbientFeedback.BP_PowerAmbientFeedback_C"))
  (for _array_element_5 _outactors_5
    (set `/Game/ProjectEcho/Gameplay/Power/BP_PowerAmbientFeedback.bPlayed` false _array_element_5))
  (bind _outactors_6 (`GameplayStatics.GetAllActorsOfClass` "/Game/ProjectEcho/Gameplay/Power/BP_VentilationUnit.BP_VentilationUnit_C"))
  (for _array_element_6 _outactors_6
    (set `/Game/ProjectEcho/Gameplay/Power/BP_VentilationUnit.bPlayed` false _array_element_6))
  (bind _outactors_7 (`GameplayStatics.GetAllActorsOfClass` "/Game/ProjectEcho/Gameplay/Power/BP_PASpeaker.BP_PASpeaker_C"))
  (for _array_element_7 _outactors_7
    (set `/Game/ProjectEcho/Gameplay/Power/BP_PASpeaker.bPlayed` false _array_element_7))
  (bind _outactors_8 (`GameplayStatics.GetAllActorsOfClass` "/Game/ProjectEcho/Gameplay/Power/BP_DistantActivityHint.BP_DistantActivityHint_C"))
  (for _array_element_8 _outactors_8
    (set `/Game/ProjectEcho/Gameplay/Power/BP_DistantActivityHint.bPlayed` false _array_element_8))
  (bind _outactors_9 (`GameplayStatics.GetAllActorsOfClass` "/Game/ProjectEcho/Gameplay/Interaction/BP_NotePickup.BP_NotePickup_C"))
  (for _array_element_9 _outactors_9
    (set `/Game/ProjectEcho/Gameplay/Interaction/BP_NotePickup.bCollected` false _array_element_9))
  (bind _outactors_10 (`GameplayStatics.GetAllActorsOfClass` "/Game/ProjectEcho/Gameplay/Power/BP_Generator.BP_Generator_C"))
  (for _array_element_10 _outactors_10
    (set `/Game/ProjectEcho/Gameplay/Power/BP_Generator.HasFuel` false _array_element_10)
    (set `/Game/ProjectEcho/Gameplay/Power/BP_Generator.PowerRestored` false _array_element_10)
    (set `/Game/ProjectEcho/Gameplay/Power/BP_Generator.GeneratorState` 0 _array_element_10))
  (`/Engine/EditorBlueprintResources/StandardMacros.IsValid` _returnvalue
    (:`Is Valid`
      (`/Game/ProjectEcho/Gameplay/Objectives/BPC_Objective.ClearObjective` _returnvalue)
      (`/Game/ProjectEcho/Gameplay/Objectives/BPC_Objective.SetObjective` _returnvalue "Investigate the main power plant"))
    (:`Is Not Valid`
      (`KismetSystemLibrary.PrintString` "[PE018] ObjectiveComponent missing on reset"))))

(fn `UserConstructionScript`)