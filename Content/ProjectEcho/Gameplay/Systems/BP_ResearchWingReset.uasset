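; Interactable reset actor ("Reset Puzzle") that returns the research wing slice to its starting state and sets the coolant bay objective shortly after BeginPlay.
; ResetWorldState sweeps actors by class, locking doors and exits, clearing light, one-shot and note flags, and resetting hints and coolant puzzles.
; ResetPlayerState then replaces the coolant bay objective that sweep sets with the research wing one.
; CompleteSliceReset repeats the Interact sequence with an extra debug print.
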(event `self.ReceiveBeginPlay`
  (bind _returnvalue (`self.GetComponentByClass` (`GameplayStatics.GetPlayerPawn` 0) "/Game/ProjectEcho/Gameplay/Objectives/BPC_Objective.BPC_Objective_C"))
  (`KismetSystemLibrary.Delay` 0.25)
  (`/Engine/EditorBlueprintResources/StandardMacros.IsValid` _returnvalue
    (:`Is Valid`
      (`/Game/ProjectEcho/Gameplay/Objectives/BPC_Objective.SetObjective` _returnvalue "Investigate the coolant bay")
      (`KismetSystemLibrary.PrintString` "[PE019] Coolant Bay ready"))
    (:`Is Not Valid`
      (`KismetSystemLibrary.PrintString` "[PE019] ObjectiveComponent missing at BeginPlay"))))

(event `self.Interact`
  (params (Interactor :type "Actor Object Reference"))
  (`self.ResetWorldState`)
  (`self.ResetPlayerState`)
  (`self.FinishPuzzleReset`))

(fn `CanInteract`
  (params (Interactor :type "Actor Object Reference"))
  (returns (ReturnValue :type Boolean))
  (return true))

(fn `CompleteSliceReset`
  (`self.ResetWorldState`)
  (`self.ResetPlayerState`)
  (`self.FinishPuzzleReset`)
  (`KismetSystemLibrary.PrintString` "[PE019] Slice world state fully reset"))

(fn `FinishPuzzleReset`
  (`KismetSystemLibrary.PrintString` "[PE020] SliceReset complete"))

(fn `GetInteractionText`
  (returns (ReturnValue :type Text))
  (return "Reset Puzzle"))

(fn `ResetPlayerState`
  (bind _returnvalue (`self.GetComponentByClass` (`GameplayStatics.GetPlayerPawn` 0) "/Game/ProjectEcho/Gameplay/Objectives/BPC_Objective.BPC_Objective_C"))
  (`/Engine/EditorBlueprintResources/StandardMacros.IsValid` _returnvalue
    (:`Is Valid`
      (`/Game/ProjectEcho/Gameplay/Objectives/BPC_Objective.SetObjective` _returnvalue "Investigate the research wing"))))

(fn `ResetWorldState`
  (bind _returnvalue (`self.GetComponentByClass` (`GameplayStatics.GetPlayerPawn` 0) "/Game/ProjectEcho/Gameplay/Objectives/BPC_Objective.BPC_Objective_C"))
  (bind _outactors (`GameplayStatics.GetAllActorsOfClass` "/Game/ProjectEcho/Gameplay/Power/BP_PoweredDoor.BP_PoweredDoor_C"))
  (for _array_element _outactors
    (set `/Game/ProjectEcho/Gameplay/Power/BP_PoweredDoor.bIsLocked` true _array_element)
    (set `/Game/ProjectEcho/Gameplay/Power/BP_PoweredDoor.bIsOpen` false _array_element))
  (bind _outactors_2 (`GameplayStatics.GetAllActorsOfClass` "/Game/ProjectEcho/Gameplay/Power/BP_SoftOpenExit.BP_SoftOpenExit_C"))
  (for _array_element_2 _outactors_2
    (set `/Game/ProjectEcho/Gameplay/Power/BP_SoftOpenExit.bIsLocked` true _array_element_2)
    (set `/Game/ProjectEcho/Gameplay/Power/BP_SoftOpenExit.bIsOpen` false _array_element_2))
  (bind _outactors_3 (`GameplayStatics.GetAllActorsOfClass` "/Game/ProjectEcho/Gameplay/Power/BP_EmergencyLight.BP_EmergencyLight_C"))
  (for _array_element_3 _outactors_3
    (set `/Game/ProjectEcho/Gameplay/Power/BP_EmergencyLight.bPoweredOn` false _array_element_3))
  (bind _outactors_4 (`GameplayStatics.GetAllActorsOfClass` "/Game/ProjectEcho/Gameplay/Power/BP_WitnessSilhouetteHint.BP_WitnessSilhouetteHint_C"))
  (for _array_element_4 _outactors_4
    (`/Game/ProjectEcho/Gameplay/Power/BP_WitnessSilhouetteHint.ResetPresence` _array_element_4))
  (bind _outactors_5 (`GameplayStatics.GetAllActorsOfClass` "/Game/ProjectEcho/Gameplay/Power/BP_PowerAmbientFeedback.BP_PowerAmbientFeedback_C"))
  (for _array_element_5 _outactors_5
    (set `/Game/ProjectEcho/Gameplay/Power/BP_PowerAmbientFeedback.bPlayed` false _array_element_5))
  (bind _outactors_6 (`GameplayStatics.GetAllActorsOfClass` "/Game/ProjectEcho/Gameplay/Power/BP_VentilationUnit.BP_VentilationUnit_C"))
  (for _array_element_6 _outactors_6
    (set `/Game/ProjectEcho/Gameplay/Power/BP_VentilationUnit.bPlayed` false _array_element_6))
  (bind _outactors_7 (`GameplayStatics.GetAllActorsOfClass` "/Game/ProjectEcho/Gameplay/Power/BP_PASpeaker.BP_PASpeaker_C"))
  (for _array_element_7 _outactors_7
    (set `/Game/ProjectEcho/Gameplay/Power/BP_PASpeaker.bPlayed` false _array_element_7))
  (bind _outactors_8 (`GameplayStatics.GetAllActorsOfClass` "/Game/ProjectEcho/Gameplay/Power/BP_DistantActivityHint.BP_DistantActivityHint_C"))
  (for _array_element_8 _outactors_8
    (set `/Game/ProjectEcho/Gameplay/Power/BP_DistantActivityHint.bPlayed` false _array_element_8))
  (bind _outactors_9 (`GameplayStatics.GetAllActorsOfClass` "/Game/ProjectEcho/Gameplay/Interaction/BP_NotePickup.BP_NotePickup_C"))
  (for _array_element_9 _outactors_9
    (set `/Game/ProjectEcho/Gameplay/Interaction/BP_NotePickup.bCollected` false _array_element_9))
  (bind _outactors_10 (`GameplayStatics.GetAllActorsOfClass` "/Game/ProjectEcho/Gameplay/Puzzle/BP_CoolantLoopPuzzle.BP_CoolantLoopPuzzle_C"))
  (for _array_element_10 _outactors_10
    (`/Game/ProjectEcho/Gameplay/Puzzle/BP_CoolantLoopPuzzle.ResetValveStates` _array_element_10)
    (`/Game/ProjectEcho/Gameplay/Puzzle/BP_PuzzleBase.ResetPuzzle` _array_element_10))
  (`/Engine/EditorBlueprintResources/StandardMacros.IsValid` _returnvalue
    (:`Is Valid`
      (`/Game/ProjectEcho/Gameplay/Objectives/BPC_Objective.ClearObjective` _returnvalue)
      (`/Game/ProjectEcho/Gameplay/Objectives/BPC_Objective.SetObjective` _returnvalue "Investigate the coolant bay"))
    (:`Is Not Valid`
      (`KismetSystemLibrary.PrintString` "[PE019] ObjectiveComponent missing on reset"))))

(fn `UserConstructionScript`)