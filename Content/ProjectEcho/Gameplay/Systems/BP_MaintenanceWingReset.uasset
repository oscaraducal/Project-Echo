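; Interactable reset button, part of the Maintenance Wing systems, that resets an assigned puzzle.
; Interact calls ResetPuzzle on TargetPuzzle, logging a message instead if none is valid.
; After a reset, the RespawnFuse option spawns a new fuse pickup at FuseSpawnPoint, falling back to the button's own transform.
; Interaction is always allowed and shows a "Reset Puzzle" prompt.
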(event `self.Interact`
  (params (Interactor :type "Actor Object Reference"))
  (bind _fusespawnpoint (`self.FuseSpawnPoint`))
  (bind _targetpuzzle (`self.TargetPuzzle`))
  (`/Engine/EditorBlueprintResources/StandardMacros.IsValid` _targetpuzzle
    (:`Is Valid`
      (`/Game/ProjectEcho/Gameplay/Puzzle/BP_PuzzleBase.ResetPuzzle` _targetpuzzle)
      (`KismetSystemLibrary.PrintString` "[PE015] Reset button -> ResetPuzzle")
      (if (`self.bRespawnFuse`)
        (`/Engine/EditorBlueprintResources/StandardMacros.IsValid` _fusespawnpoint
          (:`Is Valid`
            (`|SpawnActorFromClass` "/Game/ProjectEcho/Gameplay/Puzzle/BP_FusePickup.BP_FusePickup_C" (`self.GetTransform` _fusespawnpoint) "AlwaysSpawn" "MultiplyWithRoot" null null)
            (`KismetSystemLibrary.PrintString` "[PE015] Fuse respawned at spawn point"))
          (:`Is Not Valid`
            (`|SpawnActorFromClass` "/Game/ProjectEcho/Gameplay/Puzzle/BP_FusePickup.BP_FusePickup_C" (`self.GetTransform`) "AlwaysSpawn" "MultiplyWithRoot" null null)
            (`KismetSystemLibrary.PrintString` "[PE015] Fuse respawned at reset button")))))
    (:`Is Not Valid`
      (`KismetSystemLibrary.PrintString` "[PE015] Reset button has no TargetPuzzle"))))

(fn `CanInteract`
  (params (Interactor :type "Actor Object Reference"))
  (returns (ReturnValue :type Boolean))
  (return true))

(fn `GetInteractionText`
  (returns (ReturnValue :type Text))
  (return "Reset Puzzle"))

(fn `UserConstructionScript`)