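; BP_MedicalWingReset is an interactable puzzle reset, always usable under the "Reset Puzzle" prompt.
; Interacting calls world-state reset, player-state reset and a finishing step in sequence.
; On BeginPlay, after a short delay, it sets the player's BPC_Objective to investigate the coolant bay and prints a debug message, or reports the component missing.
; Despite the Medical Wing name, its objective and log text refer to the Coolant Bay.
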(event `self.ReceiveBeginPlay`
  (bind _returnvalue (`self.GetComponentByClass` (`GameplayStatics.GetPlayerPawn` 0) "/Game/ProjectEcho/Gameplay/Objectives/BPC_Objective.BPC_Objective_C"))
  (`KismetSystemLibrary.Delay` 0.25)
  (`/Engine/EditorBlueprintResources/StandardMacros.IsValid` _returnvalue
    (:`Is Valid`
      (`/Game/ProjectEcho/Gameplay/Objectives/BPC_Objective.SetObjective` _returnvalue "Investigate the coolant bay")
      (`KismetSystemLibrary.PrintString` "[PE019] Coolant Bay ready"))
    (:`Is Not Valid`
      (`KismetSystemLibrary.PrintString` "[PE019] ObjectiveComponent missing at BeginPlay"))))

(event `self.Interact`
  (params (Interactor :type "Actor Object Reference"))
  (`self.ResetWorldState`)
  (`self.ResetPlayerState`)
  (`self.FinishPuzzleReset`))

(fn `CanInteract`
  (params (Interactor :type "Actor Object Reference"))
  (returns (ReturnValue :type Boolean))
  (return true))

(fn `GetInteractionText`
  (returns (ReturnValue :type Text))
  (return "Reset Puzzle"))

(fn `UserConstructionScript`)