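; Emergency light actor that starts unpowered and simulates a flickering start-up when power is restored.
; OnPowerRestored runs short delays with debug prints for the flicker, then sets PoweredOn unless IsBroken marks it as failed.
; Only state and log output change; no light component is driven.
; The BPI_PowerReceiver_OnPowerRestored event is empty and does not call the OnPowerRestored sequence.
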(event `self.ReceiveBeginPlay`
  (set `self.bPoweredOn` false)
  (`KismetSystemLibrary.PrintString` "[PE011] EmergencyLight offline"))

(event `OnPowerRestored`
  (`KismetSystemLibrary.PrintString` "[PE011] EmergencyLight power restore start")
  (`KismetSystemLibrary.Delay` 0.15)
  (`KismetSystemLibrary.PrintString` "[PE011] EmergencyLight flicker 1")
  (`KismetSystemLibrary.Delay` 0.1)
  (`KismetSystemLibrary.PrintString` "[PE011] EmergencyLight flicker 2")
  (`KismetSystemLibrary.Delay` 0.15)
  (if (`self.bIsBroken`)
    (set `self.bPoweredOn` false)
    (`KismetSystemLibrary.PrintString` "[PE011] EmergencyLight FAILED (broken)")
    (else
      (set `self.bPoweredOn` true)
      (`KismetSystemLibrary.PrintString` "[PE011] EmergencyLight ON"))))

(event `BPI_PowerReceiver_OnPowerRestored`)

(fn `UserConstructionScript`)