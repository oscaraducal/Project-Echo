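; BP_VentilationUnit is a power-system actor that represents a ventilation unit coming online when power is restored.
; It logs an idle state on BeginPlay, then its OnPowerRestored event runs a one-shot startup sequence guarded by the Played flag.
; The sequence is placeholder feedback only, printing staged startup, airflow and online messages separated by short delays, with no audio, visuals or movement.
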(event `self.ReceiveBeginPlay`
  (set `self.bPlayed` false)
  (`KismetSystemLibrary.PrintString` "[PE012] VentilationUnit idle"))

(event `OnPowerRestored`
  (if (not (`self.bPlayed`))
    (set `self.bPlayed` true)
    (`KismetSystemLibrary.PrintString` "[PE012][Vent] Soft mechanical start")
    (`KismetSystemLibrary.Delay` 0.35)
    (`KismetSystemLibrary.PrintString` "[PE012][Vent] Airflow rising through ducts")
    (`KismetSystemLibrary.Delay` 0.25)
    (`KismetSystemLibrary.PrintString` "[PE012][Vent] Ventilation online")))

(fn `UserConstructionScript`)