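; Witness silhouette scare that briefly shows a figure, described in debug text as on the exit path, after power is restored.
; OnPowerRestored runs once via a Played flag, using chained Delays to reveal SilhouetteMesh and HorrorLight, then hide both.
; Debug prints stand in for the narration and sound beats.
; BeginPlay starts it hidden; ResetPresence re-arms it, with a near-duplicate ResetPresence0 function that also sets hidden-in-game.
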(event `self.ReceiveBeginPlay`
  (set `self.bPlayed` false)
  (`SceneComponent.SetVisibility` (`self.SilhouetteMesh`) false true)
  (`LightComponent.SetIntensity` (`self.HorrorLight`) 0.0)
  (`KismetSystemLibrary.PrintString` "[PE017A] WitnessPresence hidden until power"))

(event `OnPowerRestored`
  (if (not (`self.bPlayed`))
    (set `self.bPlayed` true)
    (`KismetSystemLibrary.Delay` 1.2)
    (`KismetSystemLibrary.PrintString` "[PE017A][Witness] Somewhere ahead — the dark feels watched")
    (`KismetSystemLibrary.Delay` 0.8)
    (`SceneComponent.SetVisibility` (`self.SilhouetteMesh`) true true)
    (`LightComponent.SetIntensity` (`self.HorrorLight`) 350.0)
    (`KismetSystemLibrary.PrintString` "[PE017A][Witness] A cold silhouette holds still on the exit path")
    (`KismetSystemLibrary.Delay` 1.6)
    (`KismetSystemLibrary.PrintString` "[PE017A][Witness] Distorted hush / metal breath — then nothing")
    (`KismetSystemLibrary.Delay` 0.7)
    (`SceneComponent.SetVisibility` (`self.SilhouetteMesh`) false true)
    (`LightComponent.SetIntensity` (`self.HorrorLight`) 0.0)
    (`KismetSystemLibrary.PrintString` "[PE017A][Witness] Gone. The exit still waits.")))

(event `ResetPresence`
  (set `self.bPlayed` false)
  (`SceneComponent.SetVisibility` (`self.SilhouetteMesh`) false true)
  (`LightComponent.SetIntensity` (`self.HorrorLight`) 0.0)
  (`KismetSystemLibrary.PrintString` "[PE017A] WitnessPresence reset"))

(fn `ResetPresence_0`
  (set `self.bPlayed` false)
  (`SceneComponent.SetHiddenInGame` (`self.SilhouetteMesh`) true true)
  (`SceneComponent.SetVisibility` (`self.SilhouetteMesh`) false true)
  (`LightComponent.SetIntensity` (`self.HorrorLight`) 0.0)
  (`KismetSystemLibrary.PrintString` "[PE017A] WitnessPresence reset"))

(fn `UserConstructionScript`)