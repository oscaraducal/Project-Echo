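; BP_DistantActivityHint is a one-shot actor that hints at activity elsewhere in the facility after power is restored.
; BeginPlay resets a Played flag, and OnPowerRestored checks it so the sequence runs only once.
; After short delays it prints two staged debug messages describing distant shifting and a door settling, with no audio or visual effects in the graph.
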(event `self.ReceiveBeginPlay`
  (set `self.bPlayed` false)
  (`KismetSystemLibrary.PrintString` "[PE012] DistantActivityHint idle"))

(event `OnPowerRestored`
  (if (not (`self.bPlayed`))
    (set `self.bPlayed` true)
    (`KismetSystemLibrary.Delay` 1.2)
    (`KismetSystemLibrary.PrintString` "[PE012][Distant] Something shifts elsewhere in the facility")
    (`KismetSystemLibrary.Delay` 0.3)
    (`KismetSystemLibrary.PrintString` "[PE012][Distant] A distant door or hatch settles once")))

(fn `UserConstructionScript`)