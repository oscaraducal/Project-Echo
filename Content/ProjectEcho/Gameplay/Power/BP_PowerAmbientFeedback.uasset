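; Power-restoration ambient feedback Blueprint that stands in for the facility's audio response when power returns.
; OnPowerRestored runs once, guarded by a Played flag, and steps through a short delayed sequence of narrated cues from relay snap to the returning room bed.
; The cues are only PrintString messages tagged as audio; no sounds are played, and nothing in this graph calls the event.
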(event `self.ReceiveBeginPlay`)

(event `OnPowerRestored`
  (if (not (`self.bPlayed`))
    (set `self.bPlayed` true)
    (`KismetSystemLibrary.PrintString` "[PE017A][Audio] Relay bank snaps — aux bus live")
    (`KismetSystemLibrary.Delay` 0.35)
    (`KismetSystemLibrary.PrintString` "[PE017A][Audio] Electrical hum rises through the conduit")
    (`KismetSystemLibrary.Delay` 0.45)
    (`KismetSystemLibrary.PrintString` "[PE017A][Audio] Ventilation spooling — metal breath in the ducts")
    (`KismetSystemLibrary.Delay` 0.4)
    (`KismetSystemLibrary.PrintString` "[PE017A][Audio] Distant pipe knock / settling steel")
    (`KismetSystemLibrary.Delay` 0.35)
    (`KismetSystemLibrary.PrintString` "[PE017A][Audio] Facility bed returns — thin fluorescent buzz")
    (`KismetSystemLibrary.PrintString` "[PE017A][Audio] Power restored. The wing feels awake.")))

(fn `UserConstructionScript`)