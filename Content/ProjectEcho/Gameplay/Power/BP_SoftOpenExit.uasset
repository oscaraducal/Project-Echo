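; BP_SoftOpenExit is an exit that stays locked until power is restored and can then send the player to another level.
; It starts locked on BeginPlay, and OnPowerRestored clears the lock.
; Interact reports a pressure interlock while locked; once unlocked, it opens once and, if TravelOnOpen is set, loads SoftOpenLevelName.
; Opening only sets state and prints debug messages, with no visual or collision change.
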(event `self.ReceiveBeginPlay`
  (set `self.bIsLocked` true)
  (set `self.bIsOpen` false)
  (`KismetSystemLibrary.PrintString` "[PE019] SoftOpenExit locked"))

(event `OnPowerRestored`
  (set `self.bIsLocked` false)
  (`KismetSystemLibrary.PrintString` "[PE019] SoftOpenExit UNLOCKED"))

(event `self.Interact`
  (params (Interactor :type "Actor Object Reference"))
  (if (`self.bIsLocked`)
    (`KismetSystemLibrary.PrintString` "[PE019] Exit locked - pressure interlock"))
  (if (not (`self.bIsLocked`))
    (if (not (`self.bIsOpen`))
      (set `self.bIsOpen` true)
      (`KismetSystemLibrary.PrintString` "[PE019] Exit OPEN")
      (if (`self.bTravelOnOpen`)
        (`GameplayStatics.OpenLevel` (`self.SoftOpenLevelName`)))
      (else
        (`KismetSystemLibrary.PrintString` "[PE019] Exit already open")))))

(fn `UserConstructionScript`
  (`parent.UserConstructionScript`))