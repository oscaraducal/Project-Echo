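; BPC_Objective is a component that tracks the current objective text and shows on-screen notifications when it is set or completed.
; SetObjective stores the text and shows an "updated" banner; CompleteObjective shows a "complete" banner and then clears it.
; Each banner replaces any active WBP_Objective widget with a new one for the first player and restarts a timer that removes it after DisplayDuration.
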(fn `ClearObjective`
  (set `self.CurrentObjective` "")
  (`KismetSystemLibrary.PrintString` "[PE009] Objective cleared" true true (struct :`G` 0.66 :`B` 1.0 :`A` 1.0) 3.0))

(fn `CompleteObjective`
  (`self.ShowObjectiveUI` "OBJECTIVE COMPLETE" (`self.CurrentObjective`))
  (`self.ClearObjective`)
  (`KismetSystemLibrary.PrintString` "[PE009] Objective complete" true true (struct :`G` 0.66 :`B` 1.0 :`A` 1.0) 3.0))

(fn `GetCurrentObjective`
  (returns (ReturnValue :type Text))
  (return (`self.CurrentObjective`)))

(fn `HideObjectiveUI`
  (bind _activeobjectivewidget (`self.ActiveObjectiveWidget`))
  (`/Engine/EditorBlueprintResources/StandardMacros.IsValid` _activeobjectivewidget
    (:`Is Valid`
      (`Widget.RemoveFromParent` _activeobjectivewidget)
      (set `self.ActiveObjectiveWidget` null))))

(fn `SetObjective`
  (params (NewObjective :type Text))
  (set `self.CurrentObjective` NewObjective)
  (`self.ShowObjectiveUI` "OBJECTIVE UPDATED" NewObjective)
  (`KismetSystemLibrary.PrintString` "[PE009] Objective set" true true (struct :`G` 0.66 :`B` 1.0 :`A` 1.0) 3.0))

(fn `ShowObjectiveUI`
  (params (Header :type Text) (Body :type Text))
  (`KismetSystemLibrary.K2_ClearTimer` self "HideObjectiveUI")
  (`self.HideObjectiveUI`)
  (bind _returnvalue (`|CreateWidget` "/Game/ProjectEcho/UI/WBP_Objective.WBP_Objective_C" (`GameplayStatics.GetPlayerController` 0)))
  (`/Game/ProjectEcho/UI/WBP_Objective.Setup` _returnvalue Header Body)
  (`UserWidget.AddToViewport` _returnvalue 0)
  (set `self.ActiveObjectiveWidget` _returnvalue)
  (`KismetSystemLibrary.K2_SetTimer` self "HideObjectiveUI" (`self.DisplayDuration`))
  (`KismetSystemLibrary.PrintString` "[PE009] Objective UI shown" true true (struct :`G` 0.66 :`B` 1.0 :`A` 1.0) 3.0))