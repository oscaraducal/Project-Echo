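; Interactable door actor that swings open and closed when the player interacts with it.
; Interact flips IsOpen and instantly rotates the whole actor 90 degrees of local yaw in the matching direction, with no animation.
; GetInteractionText returns an Open or Close prompt from the current state, and CanInteract always allows interaction.
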(event `/Game/ProjectEcho/Gameplay/Interaction/BPI_Interactable.Interact`
  (params (Interactor :type "Actor Object Reference"))
  (bind _returnvalue (not (`self.IsOpen`)))
  (set `self.IsOpen` _returnvalue)
  (if _returnvalue
    (`self.K2_AddActorLocalRotation` (`KismetMathLibrary.MakeRotator` 0.0 0.0 90.0))
    (else
      (`self.K2_AddActorLocalRotation` (`KismetMathLibrary.MakeRotator` 0.0 0.0 -90.0)))))

(fn `CanInteract`
  (params (Interactor :type "Actor Object Reference"))
  (returns (ReturnValue :type Boolean))
  (return true))

(fn `GetInteractionText`
  (returns (ReturnValue :type Text))
  (if (`self.IsOpen`)
    (return "Close")
    (else
      (return "Open"))))

(fn `UserConstructionScript`)