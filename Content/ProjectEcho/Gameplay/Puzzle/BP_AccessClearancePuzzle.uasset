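; Access clearance puzzle actor by name, but its live content presents a coolant manifold with valves to equalize.
; Interact only prints a debug hint to use the labeled valves, and GetInteractionText switches its prompt on the Solved flag.
; No live logic here sets Solved.
; The EventGraph also holds unreachable leftovers: repeated fuse-panel logic using inventory, objective and puzzle-state calls, plus item pickup snippets.
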(event `self.ReceiveBeginPlay`
  (`parent.ReceiveBeginPlay`))

(event `self.Interact`
  (params (Interactor :type "Actor Object Reference"))
  (`KismetSystemLibrary.PrintString` "[PE019] Use the labeled coolant valves"))

(fn `GetInteractionText`
  (returns (ReturnValue :type Text))
  (if (`self.bSolved`)
    (return "Coolant loop equalized")
    (else
      (return "COOLANT MANIFOLD - equalize labeled valves"))))

(fn `UserConstructionScript`
  (`parent.UserConstructionScript`))