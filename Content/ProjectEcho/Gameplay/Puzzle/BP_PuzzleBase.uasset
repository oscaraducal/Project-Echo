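; Base puzzle Blueprint that tracks activation, solved state and reset, broadcasting each change through event dispatchers.
; A byte state advances through activation and solve stages, with optional auto-activation on BeginPlay and reset.
; MarkSolved updates the player's BPC_Objective, then notifies world targets via BPI_PowerReceiver and optionally every BP_PowerManager by PuzzleID.
; Interaction is allowed only while active and unsolved; Interact is empty and FailPuzzle is a stub.
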(event `self.ReceiveBeginPlay`
  (bind _returnvalue (`self.GetComponentByClass` (`GameplayStatics.GetPlayerPawn` 0) "/Game/ProjectEcho/Gameplay/Objectives/BPC_Objective.BPC_Objective_C"))
  (set `self.CurrentState` 1)
  (`self.OnPuzzleStateChanged` 1)
  (`KismetSystemLibrary.PrintString` "[PE015] PuzzleBase ready" true true (struct :`G` 0.66 :`B` 1.0 :`A` 1.0) 2.0)
  (if (`self.bAutoActivateOnBeginPlay`)
    (if (not (`self.bSolved`))
      (set `self.bIsActive` true)
      (set `self.CurrentState` 2)
      (`self.OnPuzzleStateChanged` 2)
      (`self.OnPuzzleStarted`)
      (`KismetSystemLibrary.PrintString` "[PE015] Puzzle activated" true true (struct :`G` 0.66 :`B` 1.0 :`A` 1.0) 2.0)
      (set `self.CurrentState` 3)
      (`self.OnPuzzleStateChanged` 3)))
  (if (not (`KismetStringLibrary.IsEmpty` (`self.ObjectiveOnAvailable`)))
    (`/Engine/EditorBlueprintResources/StandardMacros.IsValid` _returnvalue
      (:`Is Valid`
        (`/Game/ProjectEcho/Gameplay/Objectives/BPC_Objective.SetObjective` _returnvalue (`KismetTextLibrary.Conv_StringToText` (`self.ObjectiveOnAvailable`))))
      (:`Is Not Valid`
        (`KismetSystemLibrary.PrintString` "[PE015] Objective component missing at BeginPlay" true true (struct :`G` 0.66 :`B` 1.0 :`A` 1.0) 1.0)))))

(event `self.Interact`
  (params (Interactor :type "Actor Object Reference")))

(fn `Activate`
  (if (`self.bSolved`)
    (`KismetSystemLibrary.PrintString` "[PE015] Activate ignored - already solved" true true (struct :`G` 0.66 :`B` 1.0 :`A` 1.0) 2.0)
    (else
      (set `self.bIsActive` true)
      (set `self.CurrentState` 2)
      (`self.OnPuzzleStateChanged` 2)
      (`self.OnPuzzleStarted`)
      (`KismetSystemLibrary.PrintString` "[PE015] Puzzle activated" true true (struct :`G` 0.66 :`B` 1.0 :`A` 1.0) 2.0)
      (set `self.CurrentState` 3)
      (`self.OnPuzzleStateChanged` 3))))

(fn `CanInteract`
  (params (Interactor :type "Actor Object Reference"))
  (returns (ReturnValue :type Boolean))
  (return (and (not (`self.bSolved`)) (`self.bIsActive`))))

(fn `Deactivate`
  (set `self.bIsActive` false)
  (if (not (`self.bSolved`))
    (set `self.CurrentState` 1)
    (`self.OnPuzzleStateChanged` 1)
    (`KismetSystemLibrary.PrintString` "[PE015] Puzzle deactivated" true true (struct :`G` 0.66 :`B` 1.0 :`A` 1.0) 2.0)))

(fn `FailPuzzle`
  (`self.OnPuzzleFailed`)
  (`KismetSystemLibrary.PrintString` "[PE015] Puzzle failed (stub)" true true (struct :`G` 0.66 :`B` 1.0 :`A` 1.0) 2.0))

(fn `GetInteractionText`
  (returns (ReturnValue :type Text))
  (if (`self.bSolved`)
    (return "Solved")
    (else
      (return "Insert Fuse"))))

(fn `GetPuzzleID`
  (returns (OutPuzzleID :type Name))
  (return (`self.PuzzleID`)))

(fn `GetPuzzleState`
  (returns (State :type Byte))
  (return (`self.CurrentState`)))

(fn `IsSolved`
  (returns (bSolvedOut :type Boolean))
  (return (`self.bSolved`)))

(fn `MarkSolved`
  (if (`self.bSolved`)
    (`KismetSystemLibrary.PrintString` "[PE015] MarkSolved ignored - already solved" true true (struct :`G` 0.66 :`B` 1.0 :`A` 1.0) 2.0)
    (else
      (set `self.bSolved` true)
      (set `self.SolvedTimestamp` (`KismetSystemLibrary.GetGameTimeInSeconds`))
      (set `self.bIsActive` false)
      (set `self.CurrentState` 4)
      (`self.OnPuzzleStateChanged` 4)
      (`self.OnPuzzleSolved`)
      (`KismetSystemLibrary.PrintString` "[PE015] Puzzle solved" true true (struct :`G` 0.66 :`B` 1.0 :`A` 1.0) 3.0)
      (`self.NotifyObjectives`)
      (`self.TriggerWorldResponse`)
      (set `self.CurrentState` 5)
      (`self.OnPuzzleStateChanged` 5))))

(fn `NotifyObjectives`
  (bind _returnvalue (`self.GetComponentByClass` (`GameplayStatics.GetPlayerPawn` 0) "/Game/ProjectEcho/Gameplay/Objectives/BPC_Objective.BPC_Objective_C"))
  (`/Engine/EditorBlueprintResources/StandardMacros.IsValid` _returnvalue
    (:`Is Valid`
      (if (`self.bCompleteObjectiveOnSolve`)
        (`/Game/ProjectEcho/Gameplay/Objectives/BPC_Objective.CompleteObjective` _returnvalue))
      (if (not (`KismetStringLibrary.IsEmpty` (`self.ObjectiveOnSolved`)))
        (`/Game/ProjectEcho/Gameplay/Objectives/BPC_Objective.SetObjective` _returnvalue (`KismetTextLibrary.Conv_StringToText` (`self.ObjectiveOnSolved`)))
        (`KismetSystemLibrary.PrintString` "[PE015] Objective updated on puzzle solve" true true (struct :`G` 0.66 :`B` 1.0 :`A` 1.0) 2.0)))
    (:`Is Not Valid`
      (`KismetSystemLibrary.PrintString` "[PE015] BPC_Objective missing on pawn" true true (struct :`G` 0.66 :`B` 1.0 :`A` 1.0) 2.0))))

(fn `ResetPuzzle`
  (set `self.bSolved` false)
  (set `self.SolvedTimestamp` 0.0)
  (set `self.bIsActive` false)
  (set `self.CurrentState` 1)
  (`self.OnPuzzleStateChanged` 1)
  (`self.OnPuzzleReset`)
  (`KismetSystemLibrary.PrintString` "[PE015] Puzzle reset" true true (struct :`G` 0.66 :`B` 1.0 :`A` 1.0) 2.0)
  (if (`self.bAutoActivateOnBeginPlay`)
    (if (not (`self.bSolved`))
      (set `self.bIsActive` true)
      (set `self.CurrentState` 2)
      (`self.OnPuzzleStateChanged` 2)
      (`self.OnPuzzleStarted`)
      (set `self.CurrentState` 3)
      (`self.OnPuzzleStateChanged` 3))))

(fn `SetPuzzleState`
  (params (NewState :type Byte))
  (set `self.CurrentState` NewState)
  (`self.OnPuzzleStateChanged` NewState)
  (`KismetSystemLibrary.PrintString` "[PE015] Puzzle state changed" true true (struct :`G` 0.66 :`B` 1.0 :`A` 1.0) 2.0))

(fn `TriggerWorldResponse`
  (for _array_element (`self.WorldResponseTargets`)
    (`/Engine/EditorBlueprintResources/StandardMacros.IsValid` _array_element
      (:`Is Valid`
        (if (`KismetSystemLibrary.DoesImplementInterface` _array_element "/Game/ProjectEcho/Gameplay/Power/BPI_PowerReceiver.BPI_PowerReceiver_C")
          (message `/Game/ProjectEcho/Gameplay/Power/BPI_PowerReceiver.OnPowerRestored` _array_element)
          (`KismetSystemLibrary.PrintString` "[PE015] Notified WorldResponseTarget via BPI_PowerReceiver" true true (struct :`G` 0.66 :`B` 1.0 :`A` 1.0) 2.0)))))
  (if (`self.bNotifyPowerOnSolve`)
    (bind _outactors (`GameplayStatics.GetAllActorsOfClass` "/Game/ProjectEcho/Gameplay/Power/BP_PowerManager.BP_PowerManager_C"))
    (for _array_element_2 _outactors
      (`/Game/ProjectEcho/Gameplay/Power/BP_PowerManager.NotifyPuzzlePowerResponse` _array_element_2 (`self.PuzzleID`)))
    (`KismetSystemLibrary.PrintString` "[PE015] Notified PowerManager of puzzle solve" true true (struct :`G` 0.66 :`B` 1.0 :`A` 1.0) 2.0)))

(fn `UserConstructionScript`)