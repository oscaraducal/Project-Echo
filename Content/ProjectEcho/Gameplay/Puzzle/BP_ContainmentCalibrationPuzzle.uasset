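; Coolant manifold puzzle, despite the containment calibration name, solved by setting labeled valves to equalize pressure; interacting with it only prints a hint.
; CheckValveSolve compares every BP_CoolantValve in the level to its target, then calls MarkSolved or, on first failure, updates the player's objective.
; ResetValveStates resets all valves and progress flags; neither function is called within this Blueprint.
; Fuse-panel and item-pickup chains in the EventGraph are disconnected leftovers that never run.
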(event `self.ReceiveBeginPlay`
  (`parent.ReceiveBeginPlay`))

(event `self.Interact`
  (params (Interactor :type "Actor Object Reference"))
  (`KismetSystemLibrary.PrintString` "[PE019] Use the labeled coolant valves"))

(fn `CheckValveSolve`
  (bind _returnvalue (`self.GetComponentByClass` (`GameplayStatics.GetPlayerPawn` 0) "/Game/ProjectEcho/Gameplay/Objectives/BPC_Objective.BPC_Objective_C"))
  (bind _outactors (`GameplayStatics.GetAllActorsOfClass` "/Game/ProjectEcho/Gameplay/Puzzle/BP_CoolantValve.BP_CoolantValve_C"))
  (set `self.bCheckAllMatch` true)
  (for _array_element _outactors
    (if (not (== (`/Game/ProjectEcho/Gameplay/Puzzle/BP_CoolantValve.bIsOpen` _array_element) (`/Game/ProjectEcho/Gameplay/Puzzle/BP_CoolantValve.bTargetOpen` _array_element)))
      (set `self.bCheckAllMatch` false)))
  (if (`self.bCheckAllMatch`)
    (`KismetSystemLibrary.PrintString` "[PE019] Coolant pressure equalized")
    (`self.MarkSolved`)
    (else
      (`KismetSystemLibrary.PrintString` "[PE019] Pressure unequal - hatch remains sealed")
      (if (not (`self.bProgressObjectiveSet`))
        (set `self.bProgressObjectiveSet` true)
        (`/Engine/EditorBlueprintResources/StandardMacros.IsValid` _returnvalue
          (:`Is Valid`
            (`/Game/ProjectEcho/Gameplay/Objectives/BPC_Objective.SetObjective` _returnvalue "Open the pressure hatch path")))))))

(fn `GetInteractionText`
  (returns (ReturnValue :type Text))
  (if (`self.bSolved`)
    (return "Coolant loop equalized")
    (else
      (return "COOLANT MANIFOLD - equalize labeled valves"))))

(fn `ResetValveStates`
  (bind _outactors (`GameplayStatics.GetAllActorsOfClass` "/Game/ProjectEcho/Gameplay/Puzzle/BP_CoolantValve.BP_CoolantValve_C"))
  (for _array_element _outactors
    (`/Game/ProjectEcho/Gameplay/Puzzle/BP_CoolantValve.ResetValve` _array_element))
  (set `self.bProgressObjectiveSet` false)
  (set `self.bCheckAllMatch` false)
  (`KismetSystemLibrary.PrintString` "[PE019] Valve states reset"))

(fn `UserConstructionScript`
  (`parent.UserConstructionScript`))