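; BP_CalibrationStation is an interactable coolant valve for a valve puzzle, starting open or closed according to StartOpen.
; Interacting flips IsOpen and asks OwningPuzzle to run CheckValveSolve, but is locked once that puzzle is solved; without an owning puzzle it simply toggles.
; ResetValve restores the starting state, and the interaction prompt follows the current state.
; Feedback is debug print strings only.
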(event `self.ReceiveBeginPlay`
  (set `self.bIsOpen` (`self.bStartOpen`))
  (`KismetSystemLibrary.PrintString` "[PE019] Coolant valve ready"))

(event `self.Interact`
  (params (Interactor :type "Actor Object Reference"))
  (bind _owningpuzzle (`self.OwningPuzzle`))
  (`/Engine/EditorBlueprintResources/StandardMacros.IsValid` _owningpuzzle
    (:`Is Valid`
      (if (`/Game/ProjectEcho/Gameplay/Puzzle/BP_PuzzleBase.bSolved` _owningpuzzle)
        (`KismetSystemLibrary.PrintString` "[PE019] Coolant loop already equalized"))
      (if (not (`/Game/ProjectEcho/Gameplay/Puzzle/BP_PuzzleBase.bSolved` _owningpuzzle))
        (set `self.bIsOpen` (not (`self.bIsOpen`)))
        (if (`self.bIsOpen`)
          (`KismetSystemLibrary.PrintString` "[PE019] Valve OPEN")
          (else
            (`KismetSystemLibrary.PrintString` "[PE019] Valve CLOSED")))
        (`/Game/ProjectEcho/Gameplay/Puzzle/BP_CoolantLoopPuzzle.CheckValveSolve` _owningpuzzle)))
    (:`Is Not Valid`
      (set `self.bIsOpen` (not (`self.bIsOpen`)))
      (`KismetSystemLibrary.PrintString` "[PE019] Valve toggled (no owning puzzle)"))))

(fn `CanInteract`
  (params (Interactor :type "Actor Object Reference"))
  (returns (ReturnValue :type Boolean))
  (return true))

(fn `GetInteractionText`
  (returns (ReturnValue :type Text))
  (if (`self.bIsOpen`)
    (return "Close coolant valve")
    (else
      (return "Open coolant valve"))))

(fn `ResetValve`
  (set `self.bIsOpen` (`self.bStartOpen`))
  (`KismetSystemLibrary.PrintString` "[PE019] Valve reset"))

(fn `UserConstructionScript`)