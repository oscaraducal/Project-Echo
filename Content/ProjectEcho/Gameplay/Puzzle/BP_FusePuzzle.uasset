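; Fuse panel puzzle actor that the player solves by interacting while carrying the required fuse item.
; Interact activates the puzzle on first use, firing state-change and started dispatchers, then checks the interactor's BPC_Inventory.
; With the item it consumes it and calls MarkSolved; without it, it sets a "Find the fuse" objective through BPC_Objective.
; Several disconnected leftover copies of this logic and of item-pickup logic never run.
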(event `self.ReceiveBeginPlay`
  (`parent.ReceiveBeginPlay`))

(event `self.Interact`
  (params (Interactor :type "Actor Object Reference"))
  (bind _returnvalue (`self.GetComponentByClass` Interactor "/Game/ProjectEcho/Gameplay/Inventory/BPC_Inventory.BPC_Inventory_C"))
  (bind _returnvalue_2 (`self.GetComponentByClass` Interactor "/Game/ProjectEcho/Gameplay/Objectives/BPC_Objective.BPC_Objective_C"))
  (bind _requireditemid (`self.RequiredItemID`))
  (set `self.CachedInteractor` Interactor)
  (if (`self.bSolved`)
    (`KismetSystemLibrary.PrintString` "[PE015] Fuse panel already solved" true true (struct :`G` 0.66 :`B` 1.0 :`A` 1.0) 2.0))
  (if (not (`self.bSolved`))
    (if (not (`self.bIsActive`))
      (set `self.bIsActive` true)
      (set `self.CurrentState` 2)
      (`self.OnPuzzleStateChanged` 2)
      (`self.OnPuzzleStarted`)
      (set `self.CurrentState` 3)
      (`self.OnPuzzleStateChanged` 3))
    (`/Engine/EditorBlueprintResources/StandardMacros.IsValid` _returnvalue
      (:`Is Valid`
        (bind _returnvalue_3 (`/Game/ProjectEcho/Gameplay/Inventory/BPC_Inventory.HasItem` _returnvalue (`KismetStringLibrary.Conv_StringToName` _requireditemid)))
        (if _returnvalue_3
          (`/Game/ProjectEcho/Gameplay/Inventory/BPC_Inventory.RemoveItem` _returnvalue (`KismetStringLibrary.Conv_StringToName` _requireditemid))
          (`KismetSystemLibrary.PrintString` "[PE015] Fuse inserted" true true (struct :`G` 0.66 :`B` 1.0 :`A` 1.0) 2.0)
          (`self.MarkSolved`)
          (else
            (`KismetSystemLibrary.PrintString` "[PE015] Fuse required" true true (struct :`G` 0.66 :`B` 1.0 :`A` 1.0) 2.0)
            (`/Engine/EditorBlueprintResources/StandardMacros.IsValid` _returnvalue_2
              (:`Is Valid`
                (`/Game/ProjectEcho/Gameplay/Objectives/BPC_Objective.SetObjective` _returnvalue_2 "Find the fuse"))))))
      (:`Is Not Valid`
        (`KismetSystemLibrary.PrintString` "[PE015] Inventory missing" true true (struct :`G` 0.66 :`B` 1.0 :`A` 1.0) 2.0)))))

(fn `UserConstructionScript`
  (`parent.UserConstructionScript`))