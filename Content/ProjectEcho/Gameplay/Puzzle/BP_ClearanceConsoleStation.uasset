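; Interactable coolant valve for a coolant loop puzzle, despite the asset's clearance console name.
; BeginPlay sets its open state from a configured start value, and Interact toggles it, then asks the owning puzzle to check for a solution.
; A solved puzzle blocks further toggling, while a valve without an owner just toggles.
; The interaction prompt follows the open state, and debug prints report each outcome.
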(event `self.ReceiveBeginPlay`
  (set `self.bIsOpen_0` (`self.bStartOpen_0`))
  (`KismetSystemLibrary.PrintString` "[PE019] Coolant valve ready"))

(event `self.Interact`
  (params (Interactor :type "Actor Object Reference"))
  (bind _owningpuzzle_0 (`self.OwningPuzzle_0`))
  (`/Engine/EditorBlueprintResources/StandardMacros.IsValid` _owningpuzzle_0
    (:`Is Valid`
      (if (`/Game/ProjectEcho/Gameplay/Puzzle/BP_PuzzleBase.bSolved` _owningpuzzle_0)
        (`KismetSystemLibrary.PrintString` "[PE019] Coolant loop already equalized"))
      (if (not (`/Game/ProjectEcho/Gameplay/Puzzle/BP_PuzzleBase.bSolved` _owningpuzzle_0))
        (set `self.bIsOpen_0` (not (`self.bIsOpen_0`)))
        (if (`self.bIsOpen_0`)
          (`KismetSystemLibrary.PrintString` "[PE019] Valve OPEN")
          (else
            (`KismetSystemLibrary.PrintString` "[PE019] Valve CLOSED")))
        (`/Game/ProjectEcho/Gameplay/Puzzle/BP_CoolantLoopPuzzle.CheckValveSolve` _owningpuzzle_0)))
    (:`Is Not Valid`
      (set `self.bIsOpen_0` (not (`self.bIsOpen_0`)))
      (`KismetSystemLibrary.PrintString` "[PE019] Valve toggled (no owning puzzle)"))))

(fn `CanInteract`
  (params (Interactor :type "Actor Object Reference"))
  (returns (ReturnValue :type Boolean))
  (return true))

(fn `GetInteractionText`
  (returns (ReturnValue :type Text))
  (if (`self.bIsOpen_0`)
    (return "Close coolant valve")
    (else
      (return "Open coolant valve"))))

(fn `UserConstructionScript`)