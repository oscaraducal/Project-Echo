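; Fuse pickup for a puzzle that, when interacted with, goes into the interactor's inventory and removes itself from the world.
; Interact finds BPC_Inventory on the interactor, adds ItemData, then updates BPC_Objective, if present, to direct the player to the panel.
; Without an inventory component it only prints a debug message and stays in place.
; Unconnected leftover copies of other pickup logic, including door-unlock and fuel can variants, never run.
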(event `self.ReceiveBeginPlay`
  (`parent.ReceiveBeginPlay`))

(event `self.Interact`
  (params (Interactor :type "Actor Object Reference"))
  (bind _returnvalue (`self.GetComponentByClass` Interactor "/Game/ProjectEcho/Gameplay/Inventory/BPC_Inventory.BPC_Inventory_C"))
  (bind _returnvalue_2 (`self.GetComponentByClass` Interactor "/Game/ProjectEcho/Gameplay/Objectives/BPC_Objective.BPC_Objective_C"))
  (`/Engine/EditorBlueprintResources/StandardMacros.IsValid` _returnvalue
    (:`Is Valid`
      (`/Game/ProjectEcho/Gameplay/Inventory/BPC_Inventory.AddItem` _returnvalue (`self.ItemData`))
      (`KismetSystemLibrary.PrintString` "[PE015] Fuse acquired" true true (struct :`G` 0.66 :`B` 1.0 :`A` 1.0) 2.0)
      (`/Engine/EditorBlueprintResources/StandardMacros.IsValid` _returnvalue_2
        (:`Is Valid`
          (`/Game/ProjectEcho/Gameplay/Objectives/BPC_Objective.SetObjective` _returnvalue_2 "Insert the fuse into the panel")
          (`self.K2_DestroyActor` self))
        (:`Is Not Valid`
          (`self.K2_DestroyActor` self))))
    (:`Is Not Valid`
      (`KismetSystemLibrary.PrintString` "[PE015] Inventory missing" true true (struct :`G` 0.66 :`B` 1.0 :`A` 1.0) 2.0))))

(fn `UserConstructionScript`
  (`parent.UserConstructionScript`))