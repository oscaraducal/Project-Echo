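; BP_FlashlightPickup is an interactable world pickup that gives the player a flashlight.
; On Interact it finds the interactor's BPC_Flashlight component, calls GiveFlashlight, and destroys itself.
; If the interactor also has a BPC_Objective component, it first sets the objective to reading the maintenance log.
; Interaction is always allowed and shows a "Pick Up Flashlight" prompt.
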(event `self.ReceiveBeginPlay`
  (`parent.ReceiveBeginPlay`))

(event `/Game/ProjectEcho/Gameplay/Interaction/BPI_Interactable.Interact`
  (params (Interactor :type "Actor Object Reference"))
  (bind _returnvalue (`self.GetComponentByClass` Interactor "/Game/ProjectEcho/Gameplay/Objectives/BPC_Objective.BPC_Objective_C"))
  (bind _returnvalue_2 (`self.GetComponentByClass` Interactor "/Game/ProjectEcho/Gameplay/Systems/BPC_Flashlight.BPC_Flashlight_C"))
  (`/Engine/EditorBlueprintResources/StandardMacros.IsValid` _returnvalue_2
    (:`Is Valid`
      (`/Game/ProjectEcho/Gameplay/Systems/BPC_Flashlight.GiveFlashlight` _returnvalue_2)
      (`/Engine/EditorBlueprintResources/StandardMacros.IsValid` _returnvalue
        (:`Is Valid`
          (`/Game/ProjectEcho/Gameplay/Objectives/BPC_Objective.SetObjective` _returnvalue "Read the maintenance log")
          (`self.K2_DestroyActor` self))
        (:`Is Not Valid`
          (`self.K2_DestroyActor` self))))))

(fn `CanInteract`
  (params (Interactor :type "Actor Object Reference"))
  (returns (ReturnValue :type Boolean))
  (return true))

(fn `GetInteractionText`
  (returns (ReturnValue :type Text))
  (return "Pick Up Flashlight"))

(fn `UserConstructionScript`
  (`parent.UserConstructionScript`))