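; BPC_Inventory is an inventory component that stores a list of item structs, each with an ID, display name and description.
; It exposes functions to add an item, remove or look one up by ItemID, check whether one exists, and return the whole list.
; Lookups scan the array linearly; removal deletes only the first match, and adding does no duplicate or capacity check.
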(fn `AddItem`
  (params (ItemData :type "/Game/ProjectEcho/Data/ST_InventoryItem Structure"))
  (`KismetArrayLibrary.Array_Add` (`self.Items`) ItemData))

(fn `GetAllItems`
  (returns (ReturnValue :type "Array of /Game/ProjectEcho/Data/ST_InventoryItem Structure"))
  (return (`self.Items`)))

(fn `GetItem`
  (params (ItemID :type Name))
  (returns (bSuccess :type Boolean) (ItemData :type "/Game/ProjectEcho/Data/ST_InventoryItem Structure"))
  (for _array_element (`self.Items`)
    (if (== (`.ItemID_9_1560B8564D229874B57D998980D96170` (break `/Game/ProjectEcho/Data/ST_InventoryItem` _array_element)) ItemID)
      (return true _array_element)))
  (return false (make `/Game/ProjectEcho/Data/ST_InventoryItem` "None")))

(fn `HasItem`
  (params (ItemID :type Name))
  (returns (ReturnValue :type Boolean))
  (for _array_element (`self.Items`)
    (if (== (`.ItemID_9_1560B8564D229874B57D998980D96170` (break `/Game/ProjectEcho/Data/ST_InventoryItem` _array_element)) ItemID)
      (return true)))
  (return false))

(fn `RemoveItem`
  (params (ItemID :type Name))
  (returns (Removed :type Boolean))
  (bind _items (`self.Items`))
  (for _index (range (+ (- (`KismetArrayLibrary.Array_Length` _items) 1) 1))
    (if (== (`.ItemID_9_1560B8564D229874B57D998980D96170` (break `/Game/ProjectEcho/Data/ST_InventoryItem` (`|GetArrayItem` _items _index))) ItemID)
      (`KismetArrayLibrary.Array_Remove` _items _index)
      (return true)))
  (return false))