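; Key item pickup actor that an interactor collects to advance the objective toward unlocking a secured door.
; On Interact, it adds its ItemData to the interactor's inventory component, then sets the objective text on the objective component if one exists, and destroys itself.
; Without a valid inventory component on the interactor, nothing happens and the pickup stays in the world.
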(event `self.ReceiveBeginPlay`
  (`parent.ReceiveBeginPlay`))

(event `/Game/ProjectEcho/Gameplay/Interaction/BPI_Interactable.Interact`
  (params (Interactor :type "Actor Object Reference"))
  (bind _returnvalue (`self.GetComponentByClass` Interactor "/Game/ProjectEcho/Gameplay/Objectives/BPC_Objective.BPC_Objective_C"))
  (bind _returnvalue_2 (`self.GetComponentByClass` Interactor "/Game/ProjectEcho/Gameplay/Inventory/BPC_Inventory.BPC_Inventory_C"))
  (`/Engine/EditorBlueprintResources/StandardMacros.IsValid` _returnvalue_2
    (:`Is Valid`
      (`/Game/ProjectEcho/Gameplay/Inventory/BPC_Inventory.AddItem` _returnvalue_2 (`self.ItemData`))
      (`/Engine/EditorBlueprintResources/StandardMacros.IsValid` _returnvalue
        (:`Is Valid`
          (`/Game/ProjectEcho/Gameplay/Objectives/BPC_Objective.SetObjective` _returnvalue "Unlock the secured door")
          (`self.K2_DestroyActor` self))
        (:`Is Not Valid`
          (`self.K2_DestroyActor` self))))))

(fn `UserConstructionScript`
  (`parent.UserConstructionScript`))